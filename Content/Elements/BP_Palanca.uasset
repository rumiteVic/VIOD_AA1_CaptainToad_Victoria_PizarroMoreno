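; BP_Palanca is an interactable lever that sends a switch message to every actor in its Llamar array.
; Box overlap binds OnInteract to the third-person character's interact event and unbinds it on exit.
; On interaction, it loops through the array, calling OnSwitchMessage, then queries ISignal's IsSwitched to play the toggle-on or toggle-off animation on each iteration.
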(event OnComponentBeginOverlap(Box)
  (params (OverlappedComponent :type Primitive%20Component%20Object%20Reference) (OtherActor :type Actor%20Object%20Reference) (OtherComp :type Primitive%20Component%20Object%20Reference) (OtherBodyIndex :type Integer) (bFromSweep :type Boolean) (SweepResult :type Hit%20Result%20Structure%20%28by%20ref%29))
  (bind _asbp_third_person_character (Utilities|Casting|CastToBP_ThirdPersonCharacter OtherActor))
  (EventDispatchers|BindEventtoOnInteract _asbp_third_person_character (delegate Custom|OnInteract)))

(event OnComponentEndOverlap(Box)
  (params (OverlappedComponent :type Primitive%20Component%20Object%20Reference) (OtherActor :type Actor%20Object%20Reference) (OtherComp :type Primitive%20Component%20Object%20Reference) (OtherBodyIndex :type Integer))
  (bind _asbp_third_person_character (Utilities|Casting|CastToBP_ThirdPersonCharacter OtherActor))
  (EventDispatchers|UnbindEventfromOnInteract _asbp_third_person_character (delegate Custom|OnInteract)))

(event Custom|OnInteract
  (for _array_element (Variables|Default|Getllamar)
    (Class|ISignalReceiver|OnSwitch(Message) _array_element)
    (bind _isswitched (Default|IsSwitched (Variables|Default|GetI_Signal)))
    (if _isswitched
      (Components|Animation|PlayAnimation (Variables|Default|GetSkeletalMesh) "/Game/Assets/lever_Anim_toggle-on.lever_Anim_toggle-on" false)
      (else
        (Components|Animation|PlayAnimation (Variables|Default|GetSkeletalMesh) "/Game/Assets/lever_Anim_toggle-off.lever_Anim_toggle-off" false)))))

(event EventBeginPlay)

(fn ConstructionScript)