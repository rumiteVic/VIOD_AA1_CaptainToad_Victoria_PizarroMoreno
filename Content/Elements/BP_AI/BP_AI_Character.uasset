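; AI-controlled character that senses targets, can take damage and drops coins on death.
; Perception writes the sensed actor to the blackboard's SeenActor key and saves its own location, then clears the key and walks back there when sensing fails.
; Capsule overlap with "player"-tagged components toggles CanAttack and halts movement on contact.
; Damage feeds HealthSystem; death stops the brain logic, spawns a coin pickup and disables collision.
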(event OnTargetPerceptionUpdated(AIPerception)
  (params (Actor :type Actor%20Object%20Reference) (Stimulus :type AI%20Stimulus%20Structure))
  (bind _returnvalue (AI|GetBlackboard 0))
  (bind _returnvalue_2 (Utilities|Name|MakeLiteralName "SeenActor"))
  (if (.bSuccessfullySensed (Utilities|Struct|BreakAIStimulus Stimulus))
    (Utilities|FlowControl|Sequence
      (:then_0
        (bind _output_get (Variables|Default|Setreturn true))
        (if _output_get
          (Variables|Default|SetoldLocation (Transformation|GetActorLocation))
          (Variables|Default|Setreturn false)))
      (:then_1
        (AI|Components|Blackboard|SetValueasObject _returnvalue _returnvalue_2 Actor)))
    (else
      (AI|Components|Blackboard|SetValueasObject _returnvalue _returnvalue_2 0)
      (AI|AIMoveTo (Class|PawnMovementComponent|GetPawnOwner (Variables|Character|GetCharacterMovement)) (Variables|Default|GetoldLocation) 0 5.0 false
        (:then
          (Variables|Default|Setreturn false))))))

(event OnComponentBeginOverlap(CapsuleComponent)
  (params (OverlappedComponent :type Primitive%20Component%20Object%20Reference) (OtherActor :type Actor%20Object%20Reference) (OtherComp :type Primitive%20Component%20Object%20Reference) (OtherBodyIndex :type Integer) (bFromSweep :type Boolean) (SweepResult :type Hit%20Result%20Structure%20%28by%20ref%29))
  (if (Components|ComponentHasTag OtherComp "player")
    (Variables|Default|SetcanAttack true)
    (Components|Movement|StopMovementImmediately (Variables|Character|GetCharacterMovement))))

(event OnComponentEndOverlap(CapsuleComponent)
  (params (OverlappedComponent :type Primitive%20Component%20Object%20Reference) (OtherActor :type Actor%20Object%20Reference) (OtherComp :type Primitive%20Component%20Object%20Reference) (OtherBodyIndex :type Integer))
  (if (Components|ComponentHasTag OtherComp "player")
    (Variables|Default|SetcanAttack false)))

(event EventBeginPlay
  (bind _asbp_ai_controller (Utilities|Casting|CastToBP_AI_Controller (Pawn|GetController)))
  (Variables|Default|SetAs%20BP%20AI%20Controller _asbp_ai_controller))

(event EventTick
  (params (DeltaSeconds :type Float%20%28single-precision%29)))

(event EventTakeDamage
  (params (damage :type Float%20%28double-precision%29))
  (bind _returnvalue (Transformation|GetActorLocation))
  (if (not (Variables|Default|Getdied))
    (Default|RemoveHealth (Variables|Default|GetHealthSystem) damage)
    (Audio|PlaySoundatLocation "/Game/audio/CUE_Hit.CUE_Hit" _returnvalue "0, 0, 0" 1.0 1.0 0.0 0 0 0 0)
    (bind _die (Default|ShouldDie (Variables|Default|GetHealthSystem)))
    (if _die
      (Variables|Default|Setdied true)
      (AI|Logic|StopLogic (Variables|/Script/AIModule.AIController|GetBrainComponent (Variables|Default|GetAs%20BP%20AI%20Controller)) "")
      (Game|SpawnActorfromClass "/Game/Elements/BP_PickableObject/BP_PickableObject_Coins.BP_PickableObject_Coins_C" (Math|Transform|MakeTransform _returnvalue "0, 0, 0" "2.000000,2.000000,2.000000") "Undefined" "MultiplyWithRoot" 0 0)
      (Collision|SetCollisionEnabled (Variables|Character|GetMesh) "NoCollision"))))

(fn ConstructionScript)