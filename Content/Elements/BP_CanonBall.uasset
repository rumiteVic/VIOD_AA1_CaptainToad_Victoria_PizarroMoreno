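; Cannonball projectile that damages the third-person character or knocks physics objects away.
; Each tick it sweeps along the world forward axis at Speed, with a five-second lifespan set on spawn.
; On sphere overlap, it deals DamageDone to a character through I_HealthSystem, or fires a RadialForce impulse if the hit component simulates physics.
; Either hit destroys it, while other overlaps leave it flying.
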(event OnComponentBeginOverlap(Sphere1)
  (params (OverlappedComponent :type Primitive%20Component%20Object%20Reference) (OtherActor :type Actor%20Object%20Reference) (OtherComp :type Primitive%20Component%20Object%20Reference) (OtherBodyIndex :type Integer) (bFromSweep :type Boolean) (SweepResult :type Hit%20Result%20Structure%20%28by%20ref%29))
  (Utilities|FlowControl|Sequence
    (:then_0
      (bind _asbp_third_person_character (Utilities|Casting|CastToBP_ThirdPersonCharacter OtherActor))
      (if (Utilities|DoesObjectImplementInterface _asbp_third_person_character "/Game/ActorComponents/I_HealthSystem.I_HealthSystem_C")
        (Default|TakeDamage _asbp_third_person_character (Variables|Default|GetdamageDone))
        (Actor|DestroyActor :!label _label)))
    (:then_1
      (if (Physics|IsSimulatingPhysics OtherComp "None")
        (Class|RadialForceComponent|FireImpulse (Variables|Default|GetRadialForce))
        (goto _label)))))

(event EventBeginPlay
  (Actor|SetLifeSpan 5.0))

(event EventTick
  (params (DeltaSeconds :type Float%20%28single-precision%29))
  (Transformation|AddActorWorldOffset (* (* DeltaSeconds (Variables|Default|Getspeed)) (Class|KismetMathLibrary|VectorForward)) true))

(fn ConstructionScript)