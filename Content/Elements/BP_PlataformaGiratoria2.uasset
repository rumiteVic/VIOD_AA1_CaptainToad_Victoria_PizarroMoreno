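; BP_PlataformaGiratoria2 is a rotating platform that turns its Cube around the yaw axis in response to OnSwitch.
; It checks switch state through ISignal, and the PlatformA flag selects one of two timeline-driven modes.
; With PlatformA set, the Rotate timeline sets absolute yaw, playing when switched on and reversing when off.
; Otherwise, a second timeline adds yaw increments each update when switched on, with no handling for switching off.
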(event EventOnSwitch
  (bind _cube (Variables|Default|GetCube))
  (if (Variables|Default|GetplatformA)
    (bind _isswitched (Default|IsSwitched (Variables|Default|GetI_Signal)))
    (if _isswitched
      (bind _rotate (Timeline|Rotate Play)
        (:Update
          (Transformation|SetRelativeRotation _cube (Math|Rotator|MakeRotator 0.0 0.0 (.z _rotate)) false false)))
      (else
        (Timeline|Rotate Reverse)))
    (else
      (bind _isswitched_2 (Default|IsSwitched (Variables|Default|GetI_Signal)))
      (if _isswitched_2
        (bind _rotate_2 (Timeline|Timeline Play)
          (:Update
            (Transformation|AddRelativeRotation _cube (Math|Rotator|MakeRotator 0.0 0.0 (.z _rotate_2)) false false)))))))

(fn ConstructionScript)