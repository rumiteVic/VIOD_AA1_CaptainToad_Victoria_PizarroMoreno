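; Pressure-plate button interactable that signals linked objects when stepped on.
; A box overlap triggers it when a physics-simulated component meets the required mass, or when a non-simulating component belongs to the third-person character.
; On trigger it plays a switch sound, then loops through the Llamar array, sending each entry the switch message and calling the ISignal IsSwitched interface.
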(event OnComponentBeginOverlap(Box)
  (params (OverlappedComponent :type Primitive%20Component%20Object%20Reference) (OtherActor :type Actor%20Object%20Reference) (OtherComp :type Primitive%20Component%20Object%20Reference) (OtherBodyIndex :type Integer) (bFromSweep :type Boolean) (SweepResult :type Hit%20Result%20Structure%20%28by%20ref%29))
  (if (Physics|IsSimulatingPhysics OtherComp "None")
    (if (>= (Physics|GetMass OtherComp) (Variables|Default|GetrequiredMass))
      (Audio|PlaySoundatLocation "/Game/audio/CUE_Switch.CUE_Switch" (Transformation|GetActorLocation) "0, 0, 0" 1.0 1.0 0.0 0 0 0 0 :!label _label)
      (for _array_element (Variables|Default|Getllamar)
        (Class|ISignalReceiver|OnSwitch(Message) _array_element)
        (Default|IsSwitched (Variables|Default|GetI_Signal))))
    (else
      (Utilities|Casting|CastToBP_ThirdPersonCharacter OtherActor)
      (goto _label))))

(event EventTick
  (params (DeltaSeconds :type Float%20%28single-precision%29)))

(event EventBeginPlay
  (|CallParentFunction))

(fn ConstructionScript
  (|CallParentFunction))