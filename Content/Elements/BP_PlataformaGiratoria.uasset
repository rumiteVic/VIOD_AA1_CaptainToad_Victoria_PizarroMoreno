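; BP_PlataformaGiratoria is a rotating platform that reacts to a switch signal read through ISignal, with PlatformA selecting between two modes.
; In PlatformA mode it plays or reverses the Rotate timeline, but the node that would set the Cube's pitch from it is never executed.
; Otherwise, switching on plays a second timeline that adds relative pitch to the Cube each update, and switching off does nothing.
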(event EventOnSwitch
  (if (Variables|Default|GetplatformA)
    (bind _isswitched (Default|IsSwitched (Variables|Default|GetI_Signal)))
    (if _isswitched
      (bind _rotation (Timeline|Rotate Play))
      (else
        (Timeline|Rotate Reverse)))
    (else
      (bind _isswitched_2 (Default|IsSwitched (Variables|Default|GetI_Signal)))
      (if _isswitched_2
        (bind _rotation_2 (Timeline|Timeline Play)
          (:Update
            (Transformation|AddRelativeRotation (Variables|Default|GetCube) (Math|Rotator|MakeRotator 0.0 (.y _rotation_2) 0.0) false false)))))))

(fn ConstructionScript)