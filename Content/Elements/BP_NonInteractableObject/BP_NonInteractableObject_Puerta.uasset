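; Non-interactable door actor that swings open and closed by a Timeline driving the yaw of its Door component.
; OnSwitch plays or reverses the Timeline according to the ISignal switched state.
; When NormalDoor is true, Box overlaps also open and close it, sending switched on and off signals.
; Timeline updates set NormalDoor true, so overlap control is active once the door has moved.
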(event OnComponentBeginOverlap(Box)
  (params (OverlappedComponent :type Primitive%20Component%20Object%20Reference) (OtherActor :type Actor%20Object%20Reference) (OtherComp :type Primitive%20Component%20Object%20Reference) (OtherBodyIndex :type Integer) (bFromSweep :type Boolean) (SweepResult :type Hit%20Result%20Structure%20%28by%20ref%29))
  (if (Variables|Default|GetnormalDoor)
    (Default|Switchedon (Variables|Default|GetI_Signal))
    (bind _rotate (Timeline|Timeline Play)
      (:Update
        (Transformation|SetRelativeRotation (Variables|Default|Getdoor) (Math|Rotator|MakeRotator 0.0 0.0 _rotate) false false)
        (Variables|Default|SetnormalDoor true)))))

(event OnComponentEndOverlap(Box)
  (params (OverlappedComponent :type Primitive%20Component%20Object%20Reference) (OtherActor :type Actor%20Object%20Reference) (OtherComp :type Primitive%20Component%20Object%20Reference) (OtherBodyIndex :type Integer))
  (if (Variables|Default|GetnormalDoor)
    (Default|SwitchedOff (Variables|Default|GetI_Signal))
    (bind _rotate (Timeline|Timeline Reverse)
      (:Update
        (Transformation|SetRelativeRotation (Variables|Default|Getdoor) (Math|Rotator|MakeRotator 0.0 0.0 _rotate) false false)
        (Variables|Default|SetnormalDoor true)))))

(event EventBeginPlay
  (|CallParentFunction) ; This node is disabled and will not be called.\nDrag off pins to build functionality.
)

(event EventTick
  (params (DeltaSeconds :type Float%20%28single-precision%29))
  (|CallParentFunction DeltaSeconds) ; This node is disabled and will not be called.\nDrag off pins to build functionality.
)

(event Collision|EventActorBeginOverlap
  (params (OtherActor :type Actor%20Object%20Reference))
  (|CallParentFunction OtherActor) ; This node is disabled and will not be called.\nDrag off pins to build functionality.
)

(event EventOnSwitch
  (bind _isswitched (Default|IsSwitched (Variables|Default|GetI_Signal)))
  (if _isswitched
    (bind _rotate (Timeline|Timeline Play)
      (:Update
        (Transformation|SetRelativeRotation (Variables|Default|Getdoor) (Math|Rotator|MakeRotator 0.0 0.0 _rotate) false false)
        (Variables|Default|SetnormalDoor true)))
    (else
      (Timeline|Timeline Reverse))))

(fn ConstructionScript
  (|CallParentFunction))