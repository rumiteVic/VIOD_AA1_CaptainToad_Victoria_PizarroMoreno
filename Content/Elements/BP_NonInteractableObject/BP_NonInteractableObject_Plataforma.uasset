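; Non-interactable platform actor that rotates its Cube in yaw when its OnSwitch event fires, based on the ISignal switch state.
; With PlatformA set, a timeline drives the yaw forward when switched on and reverses when switched off.
; Otherwise, each switch-on captures the current world yaw and lerps relative yaw to 90 degrees beyond it, ignoring switch-off.
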(event EventBeginPlay
  (|CallParentFunction) ; This node is disabled and will not be called.\nDrag off pins to build functionality.
)

(event Collision|EventActorBeginOverlap
  (params (OtherActor :type Actor%20Object%20Reference))
  (|CallParentFunction OtherActor) ; This node is disabled and will not be called.\nDrag off pins to build functionality.
)

(event EventTick
  (params (DeltaSeconds :type Float%20%28single-precision%29))
  (|CallParentFunction DeltaSeconds) ; This node is disabled and will not be called.\nDrag off pins to build functionality.
)

(event EventOnSwitch
  (bind _cube (Variables|Default|GetCube))
  (if (Variables|Default|GetplatformA)
    (bind _isswitched (Default|IsSwitched (Variables|Default|GetI_Signal)))
    (if _isswitched
      (bind _rotate (Timeline|Timeline Play)
        (:Update
          (Transformation|SetRelativeRotation _cube (Math|Rotator|MakeRotator 0.0 0.0 (.z _rotate)) false false)))
      (else
        (Timeline|Timeline Reverse)))
    (else
      (bind _isswitched_2 (Default|IsSwitched (Variables|Default|GetI_Signal)))
      (if _isswitched_2
        (bind _output_get (Variables|Default|SetrotationStart (Transformation|GetWorldRotation (Variables|Default|GetCube))))
        (Variables|Default|SetrotationFinish (+ (.yaw _output_get) 9e+01))
        (bind _alpha (Timeline|Timeline_0 PlayFromStart)
          (:Update
            (Transformation|SetRelativeRotation _cube (Math|Rotator|MakeRotator 0.0 0.0 (Math|Float|Lerp (.yaw (Variables|Default|GetrotationStart)) (Variables|Default|GetrotationFinish) _alpha)) false false)))))))

(fn ConstructionScript
  (|CallParentFunction))