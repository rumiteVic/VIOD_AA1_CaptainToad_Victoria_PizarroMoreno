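; Elevator (Ascensor) variant of a non-interactable object that moves between two positions when it receives a switch signal.
; BeginPlay stores the actor's world location as Inicio.
; OnSwitch reads the ISignal state to play or reverse a Timeline.
; The Timeline lerps from Inicio to Final and applies the result as relative location, without sweep.
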(event EventBeginPlay
  (Variables|Default|Setinicio (Transformation|GetActorLocation)))

(event Collision|EventActorBeginOverlap
  (params (OtherActor :type Actor%20Object%20Reference))
  (|CallParentFunction OtherActor) ; This node is disabled and will not be called.\nDrag off pins to build functionality.
)

(event EventTick
  (params (DeltaSeconds :type Float%20%28single-precision%29))
  (|CallParentFunction DeltaSeconds) ; This node is disabled and will not be called.\nDrag off pins to build functionality.
)

(event EventOnSwitch
  (bind _isswitched (Default|IsSwitched (Variables|Default|GetI_Signal)))
  (if _isswitched
    (bind _alpha (Timeline|Timeline Play)
      (:Update
        (Transformation|SetActorRelativeLocation (Math|Vector|Lerp(Vector) (Variables|Default|Getinicio) (Variables|Default|Getfinal) _alpha))))
    (else
      (Timeline|Timeline Reverse))))

(fn ConstructionScript
  (|CallParentFunction))