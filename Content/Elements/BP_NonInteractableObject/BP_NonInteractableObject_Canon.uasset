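; BP_NonInteractableObject_Canon is a cannon level element that fires cannonballs automatically and repeatedly from the start of play.
; BeginPlay spawns a BP_NonInteractableObject_CanonBall at the actor's location offset by Inicio, using the actor's rotation, and plays a blast sound.
; It then waits for the Delay variable and loops back to fire again indefinitely.
; The Inicio offset is added in world space, so it does not rotate with the cannon.
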(event EventBeginPlay
  (bind _returnvalue (Transformation|GetActorLocation))
  (|CallParentFunction)
  (Game|SpawnActorfromClass "/Game/Elements/BP_NonInteractableObject/BP_NonInteractableObject_CanonBall.BP_NonInteractableObject_CanonBall_C" (Math|Transform|MakeTransform (+ (Variables|Default|Getinicio) _returnvalue) (Transformation|GetActorRotation) "1.000000,1.000000,1.000000") "Undefined" "MultiplyWithRoot" 0 0 :!label _label)
  (Audio|PlaySoundatLocation "/Game/audio/CUE_BlastCanon.CUE_BlastCanon" _returnvalue "0, 0, 0" 1.0 1.0 0.0 0 0 0 0)
  (Utilities|FlowControl|Delay (Variables|Default|Getdelay))
  (goto _label))

(event Collision|EventActorBeginOverlap
  (params (OtherActor :type Actor%20Object%20Reference))
  (|CallParentFunction OtherActor) ; This node is disabled and will not be called.\nDrag off pins to build functionality.
)

(event EventTick
  (params (DeltaSeconds :type Float%20%28single-precision%29))
  (|CallParentFunction DeltaSeconds) ; This node is disabled and will not be called.\nDrag off pins to build functionality.
)

(fn ConstructionScript
  (|CallParentFunction))