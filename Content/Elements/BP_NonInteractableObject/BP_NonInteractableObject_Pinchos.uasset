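; BP_NonInteractableObject_Pinchos is a spike hazard ("pinchos") that damages characters when they overlap its Box component.
; On overlap it casts the other actor to the player character, then to the AI character, checking each for the I_HealthSystem interface.
; The player takes DamageDone, while AI characters receive a TakeDamage call with zero damage.
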(event OnComponentBeginOverlap(Box)
  (params (OverlappedComponent :type Primitive%20Component%20Object%20Reference) (OtherActor :type Actor%20Object%20Reference) (OtherComp :type Primitive%20Component%20Object%20Reference) (OtherBodyIndex :type Integer) (bFromSweep :type Boolean) (SweepResult :type Hit%20Result%20Structure%20%28by%20ref%29))
  (Utilities|FlowControl|Sequence
    (:then_0
      (bind _asbp_third_person_character (Utilities|Casting|CastToBP_ThirdPersonCharacter OtherActor))
      (if (Utilities|DoesObjectImplementInterface _asbp_third_person_character "/Game/ActorComponents/I_HealthSystem.I_HealthSystem_C")
        (Default|TakeDamage _asbp_third_person_character (Variables|Default|GetdamageDone))))
    (:then_1
      (bind _asbp_ai_character (Utilities|Casting|CastToBP_AI_Character OtherActor))
      (if (Utilities|DoesObjectImplementInterface _asbp_ai_character "/Game/ActorComponents/I_HealthSystem.I_HealthSystem_C")
        (Default|TakeDamage _asbp_ai_character 0.0)))))

(event EventBeginPlay
  (|CallParentFunction) ; This node is disabled and will not be called.\nDrag off pins to build functionality.
)

(event Collision|EventActorBeginOverlap
  (params (OtherActor :type Actor%20Object%20Reference))
  (|CallParentFunction OtherActor) ; This node is disabled and will not be called.\nDrag off pins to build functionality.
)

(event EventTick
  (params (DeltaSeconds :type Float%20%28single-precision%29))
  (|CallParentFunction DeltaSeconds) ; This node is disabled and will not be called.\nDrag off pins to build functionality.
)

(fn ConstructionScript
  (|CallParentFunction))